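; Coupe ship Blueprint for a selectable, order-driven unit with health and ammo bar widgets.
; BeginPlay caches both bar widgets, and Tick pushes the ship's current health and ammo into them.
; On OrderMoveTo, it reads the player character's target position and, if its selection ring is visible, eases the mesh to face it, then glides there at CoupeSpeed using MoveComponentTo.
; The construction script toggles the selection ring's visibility.
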(event `self.ReceiveBeginPlay`
  ;[1 1 1] Create and Update Health Bar
  (bind _ashealth_bar (cast `/Game/Blueprints/HealthBar` (`WidgetComponent.GetUserWidgetObject` (`self.HealthBarWidget`))))
  ;[1 1 1] Create and Update Ammo Bar
  (bind _asammo_bar (cast `/Game/Blueprints/AmmoBar` (`WidgetComponent.GetUserWidgetObject` (`self.AmmoBarWidget`)))))

(event `self.ReceiveTick`
  (params (DeltaSeconds :type "Float (single-precision)"))
  ;[1 1 1] Create and Update Health Bar
  (set `/Game/Blueprints/HealthBar.Health` (`self.CoupeHealth`) (stale `self.ReceiveBeginPlay` _ashealth_bar))
  ;[1 1 1] Create and Update Ammo Bar
  (set `/Game/Blueprints/AmmoBar.Ammo` (`self.CoupeAmmo`) (stale `self.ReceiveBeginPlay` _asammo_bar)))

(event `InputAction|OrderMoveTo` :consume false
  (params (Key :type "Key Structure"))
  (bind _shipmesh (`self.ShipMesh`))
  (bind _returnvalue (`SceneComponent.K2_GetComponentLocation` (`self.ShipMesh`)))
  (bind (_returnvalue_x _returnvalue_y) (`KismetMathLibrary.BreakVector` (`KismetMathLibrary.GetDirectionUnitVector` _returnvalue (`self.CoupeTarget`))))
  (bind _returnvalue_2 (+ (`KismetMathLibrary.RadiansToDegrees` (`KismetMathLibrary.Vector_HeadingAngle` (`KismetMathLibrary.MakeVector` _returnvalue_x _returnvalue_y))) -90.0))
  ;[1 1 1] Movement
  (:`Pressed`
    (bind _asspace_player_character (cast `/Game/Blueprints/spacePlayerCharacter` (`GameplayStatics.GetPlayerCharacter` 0)))
    (bind _movetoposition (`/Game/Blueprints/spacePlayerCharacter.MoveToPosition` _asspace_player_character))
    (set `self.CoupeTarget` (`KismetMathLibrary.MakeVector` (`|GetArrayItem` _movetoposition) (`|GetArrayItem` _movetoposition 1) (`|GetArrayItem` _movetoposition 2)))
    (if (`SceneComponent.bVisible` (`self.SelectionRing`))
      (`KismetSystemLibrary.MoveComponentTo` _shipmesh _returnvalue (`KismetMathLibrary.MakeRotator` 0.0 0.0 _returnvalue_2) false true 0.5 true)
      (`KismetSystemLibrary.MoveComponentTo` _shipmesh (`self.CoupeTarget`) (`KismetMathLibrary.MakeRotator` 0.0 0.0 _returnvalue_2) false false (/ (`KismetMathLibrary.Vector_Distance` _returnvalue (`self.CoupeTarget`)) (`self.CoupeSpeed`)) true))))

(fn `UserConstructionScript`
  (`SceneComponent.ToggleVisibility` (`self.SelectionRing`) false))