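; First-person space player character that flies along the control rotation and aims a move-to point on an adjustable height plane.
; Each Tick deprojects the screen center, intersects that ray with the horizontal plane at MoveToHeight, stores MoveToPosition and draws a debug point there.
; Height inputs step MoveToHeight and, like the show input, briefly draw the plane.
; SelectShip is an empty stub, and nothing here consumes MoveToPosition.
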(event `InputAxis|MoveForward`
  (params (AxisValue :type "Float (single-precision)"))
  ;[1 1 1] Movement
  (`self.AddMovementInput` (`KismetMathLibrary.GetForwardVector` (`self.GetControlRotation`)) AxisValue))

(event `InputAxis|Turn`
  (params (AxisValue :type "Float (single-precision)"))
  ;[1 1 1] First Person Camera
  (`self.AddControllerYawInput` AxisValue))

(event `InputAxis|LookUp`
  (params (AxisValue :type "Float (single-precision)"))
  ;[1 1 1] First Person Camera
  (`self.AddControllerPitchInput` AxisValue))

(event `InputAction|ShowMoveToHeight`
  (params (Key :type "Key Structure"))
  (bind _movetovecmag (`self.MoveToVecMag`))
  (bind _movetoheight (`self.MoveToHeight`))
  (bind (_sizex _sizey) (`PlayerController.GetViewportSize` (`GameplayStatics.GetPlayerController` 0)))
  (bind (_worldlocation _worlddirection) (`PlayerController.DeprojectScreenPositionToWorld` (`GameplayStatics.GetPlayerController` 0) (`KismetMathLibrary.Conv_IntToDouble` (/ _sizex 2)) (`KismetMathLibrary.Conv_IntToDouble` (/ _sizey 2))))
  (bind (_t _intersection) (`KismetMathLibrary.LinePlaneIntersection` (`KismetMathLibrary.MakeVector` (.x _worldlocation) (.y _worldlocation) (.z _worldlocation)) (`KismetMathLibrary.MakeVector` (+ (.x _worldlocation) (* (.x _worlddirection) _movetovecmag)) (+ (.y _worldlocation) (* (.y _worlddirection) _movetovecmag)) (+ (.z _worldlocation) (* (.z _worlddirection) _movetovecmag))) (make `Plane` (`self.MoveToHeight`) 0.0 0.0 1.0)))
  ;[1 1 1] Show/Change Z-Level
  (:`Pressed`
    (`KismetSystemLibrary.DrawDebugPlane` (make `Plane` _movetoheight 0.0 0.0 1.0) (`KismetMathLibrary.MakeVector` (.x _intersection) (.y _intersection) _movetoheight) 10000.0 (struct :`R` 0.116624 :`G` 1.0 :`A` 1.0) 0.1 :!label _label)))

(event `InputAction|MoveToUp`
  (params (Key :type "Key Structure"))
  ;[1 1 1] Show/Change Z-Level
  (:`Pressed`
    (set `self.MoveToHeight` (+ (`self.MoveToHeight`) (`self.MoveToHeightInc`)))
    (goto _label)))

(event `InputAxis|MoveRight`
  (params (AxisValue :type "Float (single-precision)"))
  ;[1 1 1] Movement
  (`self.AddMovementInput` (`KismetMathLibrary.GetRightVector` (`self.GetControlRotation`)) AxisValue))

(event `InputAction|MoveToDown`
  (params (Key :type "Key Structure"))
  ;[1 1 1] Show/Change Z-Level
  (:`Pressed`
    (set `self.MoveToHeight` (- (`self.MoveToHeight`) (`self.MoveToHeightInc`)))
    (goto _label)))

(event `self.ReceiveTick`
  (params (DeltaSeconds :type "Float (single-precision)"))
  (bind _movetovecmag (`self.MoveToVecMag`))
  (bind (_sizex _sizey) (`PlayerController.GetViewportSize` (`GameplayStatics.GetPlayerController` 0)))
  (bind (_worldlocation _worlddirection) (`PlayerController.DeprojectScreenPositionToWorld` (`GameplayStatics.GetPlayerController` 0) (`KismetMathLibrary.Conv_IntToDouble` (/ _sizex 2)) (`KismetMathLibrary.Conv_IntToDouble` (/ _sizey 2))))
  (bind (_t _intersection) (`KismetMathLibrary.LinePlaneIntersection` (`KismetMathLibrary.MakeVector` (.x _worldlocation) (.y _worldlocation) (.z _worldlocation)) (`KismetMathLibrary.MakeVector` (+ (.x _worldlocation) (* (.x _worlddirection) _movetovecmag)) (+ (.y _worldlocation) (* (.y _worlddirection) _movetovecmag)) (+ (.z _worldlocation) (* (.z _worlddirection) _movetovecmag))) (make `Plane` (`self.MoveToHeight`) 0.0 0.0 1.0)))
  ;[1 1 1] Show MoveTo Position / Crosshair
  (`KismetSystemLibrary.DrawDebugPoint` (`KismetMathLibrary.MakeVector` (.x _intersection) (.y _intersection) (.z _intersection)) 5.0 (struct :`G` 1.0 :`B` 0.104671 :`A` 1.0) (* DeltaSeconds 1.01))
  (set `self.MoveToPosition` (`|MakeArray` (.x _intersection) (.y _intersection) (.z _intersection))))

(fn `SelectShip`
  (params (ShipNumber :type Integer)))

(fn `UserConstructionScript`)